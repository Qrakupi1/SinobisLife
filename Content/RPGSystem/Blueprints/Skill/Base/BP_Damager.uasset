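; BP_Damager is a short-lived skill actor that applies AoE damage and chance-based status effects to a set of hit results.
; DoDamage walks HitResult through self-calling events with tiny Delays, uncapped when MaxHit is 1 or less, otherwise stopping at MaxHit enemies.
; Each valid target within the angle range takes hit-count-scaled damage through SkillOwner and triggers OnHit.
; DamageDone reports DamagedTargets through OnAoeHitDone, then destroys the actor.
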(event `DamageDone`
  (`self.OnAoeHitDone` (`self.DamagedTargets`))
  (`self.K2_DestroyActor`))

(event `Loop`
  (bind (_min _max) (`self.GetAngle`))
  (bind _skillowner (`self.SkillOwner`))
  (bind ((`DamageType_258_ACFCC5534FFDE6843948798661995027` _damagetype) (`AttackType_373_40B0C27A44C55567BD541FA9DFEFE11C` _attacktype) (`Element_117_059CB9E0438FAA29B2D411ADBF8FC42E` _element) (`Damage_356_051999E94AC01F21023A41B864B49BC7` _damage) (`DamagePercent_357_50D9E6784A2908832B46C2B0A83D478C` _damagepercent) (`FixedDamage_358_212AAC024782C20480D70FA876ABC285` _fixeddamage) (`MultiHitCount_136_4FE79D72405666B66DD53AA3CA1C52B4` _multihitcount) (`DamageBoostPerHitCount_270_A022BECE44DBBD2E0B976AAF6159573A` _damageboostperhitcount) (`DivideDamageByHitCount_268_F4E6AF5D4E2B4CE72FD102A6484795DD` _dividedamagebyhitcount)) (break `/Game/RPGSystem/Blueprints/Structure/Skill/S_Skill` (`self.SkillInfo`)))
  (bind (_bblockinghit _binitialoverlap _time _distance _location _impactpoint _normal _impactnormal _physmat _hitactor) (`GameplayStatics.BreakHitResult` (`|GetArrayItem` (`self.HitResult`) (`self.LoopIndex`))))
  (bind (_valid _target_) (`/Game/RPGSystem/Blueprints/Interface/BPL_RPGSystem.IsValidTarget` (`self.SkillOwner`) _hitactor))
  (bind _returnvalue (`ActorComponent.GetOwner` _target_))
  ;[1 1 1] Without
  (if (> (`KismetArrayLibrary.Array_Length` (`self.HitResult`)) 0)
    (`|ExecutionSequence`
      (:`then_0`
        (`/Engine/EditorBlueprintResources/StandardMacros.IsValid` _hitactor
          (:`Is Valid`
            (if _valid
              (`/Engine/EditorBlueprintResources/StandardMacros.IsValid` _returnvalue
                (:`Is Valid`
                  (if (`/Game/RPGSystem/Blueprints/Interface/RPG_MacroLibrary.IsTargetInAngle` (- (`self.K2_GetActorLocation`) (`self.K2_GetActorLocation` _returnvalue)) _min _max (`KismetMathLibrary.GetForwardVector` (`self.K2_GetActorRotation`)))
                    (`/Game/RPGSystem/Blueprints/BPC_RPGSystem.DoDamage` _skillowner _target_ _skillowner (`/Game/RPGSystem/Blueprints/Interface/BPL_RPGSystem.DamageBoostPerCount` (`/Game/RPGSystem/Blueprints/Interface/BPL_RPGSystem.DamageDivideByCount` _damage _multihitcount _dividedamagebyhitcount) _damageboostperhitcount _multihitcount (`self.HitCount`)) _damagetype _element (`self.ImpulseInfo`) (`self.AttackBonus`) (`self.Bonus`) _impactpoint true)
                    (for _array_element (`.StatusEffectOnTarget_354_5617252545BF0402914CCEAFC0CB306A` (break `/Game/RPGSystem/Blueprints/Structure/Skill/S_Skill` (`self.SkillInfo`)))
                      (`/Engine/EditorBlueprintResources/StandardMacros.IsValid` _target_
                        (:`Is Valid`
                          (if (`/Game/RPGSystem/Blueprints/Interface/RPG_MacroLibrary.CalcChance` (`.Chance_5_6DFCE42A4E0EB39F96E094BDAD99BD4D` (break `/Game/RPGSystem/Blueprints/Structure/Skill/S_StatusEffectOnTargetEntry` _array_element)))
                            (`/Game/RPGSystem/Blueprints/BPC_RPGSystem.AddStatusEffectServer` _target_ (break `/Game/RPGSystem/Blueprints/Structure/Skill/S_StatusEffectOnTargetEntry` _array_element) 0 false (`.Damage_9_DA8AC32A4A1CB2B65B26D29920A6F9BD` (break `/Game/RPGSystem/Blueprints/Structure/Skill/S_StatusEffectOnTargetEntry` _array_element)) (`.Duration_7_D71DBA484DC99C10A27ED0B45D12862E` (break `/Game/RPGSystem/Blueprints/Structure/Skill/S_StatusEffectOnTargetEntry` _array_element)) (`self.SkillOwner`))))))
                    (`KismetArrayLibrary.Array_AddUnique` (`self.DamagedTargets`) _target_)
                    (`self.OnHit` _target_))))))))
      (:`then_1`
        (`/Engine/EditorBlueprintResources/StandardMacros.IncrementInt` (`self.LoopIndex`)
          (:`  `
            (if (< (`self.LoopIndex`) (`KismetArrayLibrary.Array_Length` (`self.HitResult`)))
              (`KismetSystemLibrary.Delay` 1e-06)
              (`self.Loop`)
              (else
                (`self.DamageDone`)))))))
    (else
      (`self.DamageDone`))))

(event `DoDamage`
  (if (<= (`self.MaxHit`) 1)
    (`self.Loop`)
    (else
      (`self.LoopMaxCount`))))

(event `LoopMaxCount`
  (bind (_min _max) (`self.GetAngle`))
  (bind _skillowner (`self.SkillOwner`))
  (bind ((`DamageType_258_ACFCC5534FFDE6843948798661995027` _damagetype) (`AttackType_373_40B0C27A44C55567BD541FA9DFEFE11C` _attacktype) (`Element_117_059CB9E0438FAA29B2D411ADBF8FC42E` _element) (`Damage_356_051999E94AC01F21023A41B864B49BC7` _damage) (`DamagePercent_357_50D9E6784A2908832B46C2B0A83D478C` _damagepercent) (`FixedDamage_358_212AAC024782C20480D70FA876ABC285` _fixeddamage) (`MultiHitCount_136_4FE79D72405666B66DD53AA3CA1C52B4` _multihitcount) (`DamageBoostPerHitCount_270_A022BECE44DBBD2E0B976AAF6159573A` _damageboostperhitcount) (`DivideDamageByHitCount_268_F4E6AF5D4E2B4CE72FD102A6484795DD` _dividedamagebyhitcount)) (break `/Game/RPGSystem/Blueprints/Structure/Skill/S_Skill` (`self.SkillInfo`)))
  (bind (_bblockinghit _binitialoverlap _time _distance _location _impactpoint _normal _impactnormal _physmat _hitactor) (`GameplayStatics.BreakHitResult` (`|GetArrayItem` (`self.HitResult`) (`self.LoopIndex`))))
  (bind (_valid _target_) (`/Game/RPGSystem/Blueprints/Interface/BPL_RPGSystem.IsValidTarget` (`self.SkillOwner`) _hitactor))
  (bind _returnvalue (`ActorComponent.GetOwner` _target_))
  ;[1 1 1] With MaxCount
  (if (> (`KismetArrayLibrary.Array_Length` (`self.HitResult`)) 0)
    (`|ExecutionSequence`
      (:`then_0`
        (`/Engine/EditorBlueprintResources/StandardMacros.IsValid` _hitactor
          (:`Is Valid`
            (if _valid
              (`/Engine/EditorBlueprintResources/StandardMacros.IsValid` _returnvalue
                (:`Is Valid`
                  (if (`/Game/RPGSystem/Blueprints/Interface/RPG_MacroLibrary.IsTargetInAngle` (- (`self.K2_GetActorLocation`) (`self.K2_GetActorLocation` _returnvalue)) _min _max (`KismetMathLibrary.GetForwardVector` (`self.K2_GetActorRotation`)))
                    (`/Engine/EditorBlueprintResources/StandardMacros.IncrementInt` (`self.EnemyHits`)
                      (:`  `
                        (`/Game/RPGSystem/Blueprints/BPC_RPGSystem.DoDamage` _skillowner _target_ _skillowner (`/Game/RPGSystem/Blueprints/Interface/BPL_RPGSystem.DamageBoostPerCount` (`/Game/RPGSystem/Blueprints/Interface/BPL_RPGSystem.DamageDivideByCount` _damage _multihitcount _dividedamagebyhitcount) _damageboostperhitcount _multihitcount (`self.HitCount`)) _damagetype _element (`self.ImpulseInfo`) (`self.AttackBonus`) (`self.Bonus`) _impactpoint false)
                        (for _array_element (`.StatusEffectOnTarget_354_5617252545BF0402914CCEAFC0CB306A` (break `/Game/RPGSystem/Blueprints/Structure/Skill/S_Skill` (`self.SkillInfo`)))
                          (`/Engine/EditorBlueprintResources/StandardMacros.IsValid` _target_
                            (:`Is Valid`
                              (if (`/Game/RPGSystem/Blueprints/Interface/RPG_MacroLibrary.CalcChance` (`.Chance_5_6DFCE42A4E0EB39F96E094BDAD99BD4D` (break `/Game/RPGSystem/Blueprints/Structure/Skill/S_StatusEffectOnTargetEntry` _array_element)))
                                (`/Game/RPGSystem/Blueprints/BPC_RPGSystem.AddStatusEffectServer` _target_ (break `/Game/RPGSystem/Blueprints/Structure/Skill/S_StatusEffectOnTargetEntry` _array_element) 0 false (`.Damage_9_DA8AC32A4A1CB2B65B26D29920A6F9BD` (break `/Game/RPGSystem/Blueprints/Structure/Skill/S_StatusEffectOnTargetEntry` _array_element)) (`.Duration_7_D71DBA484DC99C10A27ED0B45D12862E` (break `/Game/RPGSystem/Blueprints/Structure/Skill/S_StatusEffectOnTargetEntry` _array_element)) (`self.SkillOwner`))))))
                        (`KismetArrayLibrary.Array_AddUnique` (`self.DamagedTargets`) _target_)
                        (`self.OnHit` _target_))))))))))
      (:`then_1`
        (`/Engine/EditorBlueprintResources/StandardMacros.IncrementInt` (`self.LoopIndex`)
          (:`  `
            (if (< (`self.EnemyHits`) (`self.MaxHit`))
              (if (< (`self.LoopIndex`) (`KismetArrayLibrary.Array_Length` (`self.HitResult`)))
                (`KismetSystemLibrary.Delay` 0.0001)
                (`self.LoopMaxCount`)
                (else
                  (`self.DamageDone` :!label _label)))
              (else
                (goto _label)))))))
    (else
      (`self.DamageDone`))))

(fn `UserConstructionScript`)