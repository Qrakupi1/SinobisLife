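; Windstorm mage skill that plays a storm effect at a ground-snapped position and relies on inherited skill logic for its AoE hits.
; On start it caches max damage, spawns the attached storm particle for hit count times hit delay, then runs the basic skill start.
; After each AoE hit it spawns an ice-break burst, shakes the camera and re-rolls damage slightly below the maximum.
; Both effects scale with the trace radius or box length.
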(event `self.SkillStart`
  (bind ((`AttackType_373_40B0C27A44C55567BD541FA9DFEFE11C` _attacktype) (`Damage_356_051999E94AC01F21023A41B864B49BC7` _damage) (`DamagePercent_357_50D9E6784A2908832B46C2B0A83D478C` _damagepercent) (`FixedDamage_358_212AAC024782C20480D70FA876ABC285` _fixeddamage) (`StatBonus_359_3B57C4364598C5F583267DB033D55A4F` _statbonus) (`MaxDistance_368_5E7BEEB44EA06C76E03CE3B4E996DBE3` _maxdistance) (`AddRangedAttackDistance_362_6DD95E9646DD75F8043FCCB50677CC7C` _addrangedattackdistance) (`SelectLocation_366_C5CA3EA8428B46429451D2907239E860` _selectlocation) (`RequiresTarget_365_6F607FA54968B0E98F0228B2F39AC63A` _requirestarget) (`Attach_363_397EB6374CF69E70C8A6F7A50AC374EC` _attach) (`AsyncAoE_386_5C9CB04444CB3991BAFDDF8D24D390D2` _asyncaoe) (`TraceType_254_9BFE8A074B33E463AEBCF88884F007C0` _tracetype) (`AttackRangeOverwriteAI_384_6B1418ED4F34C1DDFA4866B99ECC3E31` _attackrangeoverwriteai) (`TraceSettings_239_6436F7F74F429B5E93F83AB2033EF85B` _tracesettings) (`BoxTraceSettings_251_A0617A15432F46517C736F8FD2687628` _boxtracesettings)) (break `/Game/RPGSystem/Blueprints/Structure/Skill/S_Skill` (`self.SkillInfo`)))
  (set `self.MaxDamage` _damage)
  (`self.SnapToGround`)
  (`self.SpawnParticles` "/Game/RPGSystem/Particles/P_Windstorm.P_Windstorm" (struct) (`self.K2_GetActorLocation`) (0.0 0.0 0.0) (`KismetMathLibrary.Conv_DoubleToVector` (* (/ (select `/Game/RPGSystem/Blueprints/Enum/Skill/E_SkillTraceType` _tracetype :`NewEnumerator0` (`.Radius_19_6BDBC5774B346A254DE606BFD88AD5E7` (break `/Game/RPGSystem/Blueprints/Structure/Skill/S_SkillTraceSettings` _tracesettings)) :`NewEnumerator1` (`.Length_5_6BDBC5774B346A254DE606BFD88AD5E7` (break `/Game/RPGSystem/Blueprints/Structure/Skill/S_SkillBoxTraceSettings` _boxtracesettings)) :!type "Float (double-precision)") 200.0) 0.55)) (* (`self.HitCount`) (`self.HitDelay`)) false self)
  (`self.BasicSkillStart`))

(event `self.OnAoeHitDone`
  (params (Targets :type "Array of /Game/RPGSystem/Blueprints/BPC_RPGSystem Object Reference (by ref)"))
  (bind _maxdamage (`self.MaxDamage`))
  (bind ((`AttackType_373_40B0C27A44C55567BD541FA9DFEFE11C` _attacktype) (`Damage_356_051999E94AC01F21023A41B864B49BC7` _damage) (`DamagePercent_357_50D9E6784A2908832B46C2B0A83D478C` _damagepercent) (`FixedDamage_358_212AAC024782C20480D70FA876ABC285` _fixeddamage) (`StatBonus_359_3B57C4364598C5F583267DB033D55A4F` _statbonus) (`MaxDistance_368_5E7BEEB44EA06C76E03CE3B4E996DBE3` _maxdistance) (`AddRangedAttackDistance_362_6DD95E9646DD75F8043FCCB50677CC7C` _addrangedattackdistance) (`SelectLocation_366_C5CA3EA8428B46429451D2907239E860` _selectlocation) (`RequiresTarget_365_6F607FA54968B0E98F0228B2F39AC63A` _requirestarget) (`Attach_363_397EB6374CF69E70C8A6F7A50AC374EC` _attach) (`AsyncAoE_386_5C9CB04444CB3991BAFDDF8D24D390D2` _asyncaoe) (`TraceType_254_9BFE8A074B33E463AEBCF88884F007C0` _tracetype) (`AttackRangeOverwriteAI_384_6B1418ED4F34C1DDFA4866B99ECC3E31` _attackrangeoverwriteai) (`TraceSettings_239_6436F7F74F429B5E93F83AB2033EF85B` _tracesettings) (`BoxTraceSettings_251_A0617A15432F46517C736F8FD2687628` _boxtracesettings)) (break `/Game/RPGSystem/Blueprints/Structure/Skill/S_Skill` (`self.SkillInfo`)))
  ;[1 1 1] Comment
  (`self.SpawnParticles` "/Game/RPGSystem/Particles/IBEffects/Effects/FX_Mobile/ICE/combat/P_IceTrap_Break.P_IceTrap_Break" (struct) (`self.K2_GetActorLocation`) (0.0 0.0 0.0) (`KismetMathLibrary.Conv_DoubleToVector` (* (/ (select `/Game/RPGSystem/Blueprints/Enum/Skill/E_SkillTraceType` _tracetype :`NewEnumerator0` (`.Radius_19_6BDBC5774B346A254DE606BFD88AD5E7` (break `/Game/RPGSystem/Blueprints/Structure/Skill/S_SkillTraceSettings` _tracesettings)) :`NewEnumerator1` (`.Length_5_6BDBC5774B346A254DE606BFD88AD5E7` (break `/Game/RPGSystem/Blueprints/Structure/Skill/S_SkillBoxTraceSettings` _boxtracesettings)) :!type "Float (double-precision)") 200.0) 0.55)))
  (message `/Game/RPGSystem/Blueprints/Interface/BPI_RPGSystem.DoCameraShake` (`ActorComponent.GetOwner` (`self.SkillOwner`)) "/Game/RPGSystem/Blueprints/CameraShakes/CS_ExampleShake.CS_ExampleShake_C" (`self.K2_GetActorLocation`) 0.0 2500.0 0.05 false)
  (setmembers `/Game/RPGSystem/Blueprints/Structure/Skill/S_Skill` :`StructRef` (`self.SkillInfo`) :`Damage` (`KismetMathLibrary.RandomFloatInRange` (* _maxdamage 0.98) _maxdamage)))

(fn `UserConstructionScript`
  (`parent.UserConstructionScript`))