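; BP_Skill_EarthStrikeMain is the launcher actor for the Swordman Earth Strike skill.
; On SkillStart it detaches in world space, spawns one BP_Skill_EarthStrike slightly ahead along its facing, passes on the skill data and owner, then calls SkillEnd.
; A loop for a three-way angled spread is left unconnected, so the yaw offset resolves to zero.
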(event `self.SkillStart`
  (bind (_returnvalue_roll _returnvalue_pitch _returnvalue_yaw) (`KismetMathLibrary.BreakRotator` (`self.K2_GetActorRotation`)))
  (bind _returnvalue (`KismetMathLibrary.MakeRotator` _returnvalue_roll _returnvalue_pitch (+ _returnvalue_yaw (select `bool` (> 0 1) :`false` (* 0 55.0) :`true` -55.0))))
  ;[1 1 1] Comment
  (`self.K2_DetachFromActor` "KeepWorld" "KeepWorld" "KeepWorld")
  (`|SpawnActorFromClass` "/Game/RPGSystem/Blueprints/Skill/Swordman/BP_Skill_EarthStrike.BP_Skill_EarthStrike_C" (`KismetMathLibrary.MakeTransform` (+ (`self.K2_GetActorLocation`) (* (`KismetMathLibrary.GetForwardVector` _returnvalue) 30.0)) _returnvalue) "AlwaysSpawn" "OverrideRootScale" self (`self.SkillInfo`) (`self.SkillOwner`) (`self.SkillLevel`) (`self.SkillID`) null (`self.Key`) null)
  (`self.SkillEnd`))

(fn `UserConstructionScript`
  (`parent.UserConstructionScript`))