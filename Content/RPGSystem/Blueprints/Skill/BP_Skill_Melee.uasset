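; BP_Skill_Melee is a melee basic-attack skill that applies hit reactions and knockback to enemies.
; On start it spawns a fire impact particle; on hit it turns the enemy toward the attacker, plays a hit montage and launches it using the current combo step's force.
; On end it chains any queued basic attack after a short delay.
; Hits disable enemy movement and attacking, but the re-enabling nodes are unconnected.
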(event `self.ReceiveBeginPlay`
  (`parent.ReceiveBeginPlay`))

(event `self.OnHit`
  (params (Target :type "/Game/RPGSystem/Blueprints/BPC_RPGSystem Object Reference"))
  (bind _returnvalue (`self.GetOwner`))
  (bind _skillowner (`self.SkillOwner`))
  (bind _returnvalue_2 (`self.K2_GetActorRotation` _returnvalue))
  (bind _asbp_enemy_base (cast `/Game/RPGSystem/Blueprints/AI/BP_Enemy_Base` (`ActorComponent.GetOwner` Target)))
  (bind (_success _reference) (`/Game/RPGSystem/Blueprints/Interface/BPI_RPGSystem.GetRPGSystem` _asbp_enemy_base))
  (if _success
    (`self.K2_SetActorRotation` _asbp_enemy_base (`KismetMathLibrary.FindLookAtRotation` (`self.K2_GetActorLocation` _asbp_enemy_base) (`self.K2_GetActorLocation` _returnvalue)) true)
    (set `/Game/RPGSystem/Blueprints/BPC_RPGSystem.ForceDisableMovement` true _reference)
    (set `/Game/RPGSystem/Blueprints/BPC_RPGSystem.DisableAttacking` true _reference)
    (set `/Game/RPGSystem/Blueprints/BPC_RPGSystem.HitReactionType` 0 _skillowner)
    (`Character.LaunchCharacter` _asbp_enemy_base (+ (* (`KismetMathLibrary.GetForwardVector` _returnvalue_2) (`|GetArrayItem` (`.BasicAttacksForce_397_D9547A544FAC81CF1AA71EABEB7E89AD` (break `/Game/RPGSystem/Blueprints/Structure/Skill/S_Skill` (`/Game/RPGSystem/Blueprints/BPC_RPGSystem.CurrentSkillinfo` _skillowner))) (`/Game/RPGSystem/Blueprints/BPC_RPGSystem.BasicAttackComboCount` _skillowner))) (* (`KismetMathLibrary.GetUpVector` _returnvalue_2) 100.0)) false false)
    (`Character.PlayAnimMontage` _asbp_enemy_base "/Game/AllMyData/MyAnimations/Hits/Defailt/Frank_RPG_Fighter_Hit01_Montage.Frank_RPG_Fighter_Hit01_Montage" 1.0 "None")
    (`KismetSystemLibrary.Delay` 1.0)))

(event `self.SkillStart`
  ;[1 1 1] Partilcles
  (`self.SpawnParticles` "/Game/RPGSystem/Particles/P_Impact_Player_Fire_Strong.P_Impact_Player_Fire_Strong" (`self.K2_GetActorRotation`) (`self.K2_GetActorLocation`) (* (`self.GetActorForwardVector`) 100.0) (1.0 0.4 1.0))
  (`parent.SkillStart`))

(event `self.SkillEnd`
  (bind _skillowner (`self.SkillOwner`))
  ;[1 1 1] Execute next basic attack
  (if (`/Game/RPGSystem/Blueprints/BPC_RPGSystem.NextSkillExecute` _skillowner)
    (`KismetSystemLibrary.Delay` 0.1)
    (set `/Game/RPGSystem/Blueprints/BPC_RPGSystem.NextSkillExecute` false _skillowner)
    (`/Game/RPGSystem/Blueprints/BPC_RPGSystem.BasicAttack` _skillowner (`/Game/RPGSystem/Blueprints/BPC_RPGSystem.NextSkillKey` _skillowner))))

(fn `UserConstructionScript`
  (`parent.UserConstructionScript`))