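; Whirlwind skill Blueprint (WirbelWind) in the RPG system, extending a parent skill class.
; On SkillStart it spawns the P_WirbelWind particle effect attached to itself with an effectively unlimited destroy timer, then calls the parent's start logic.
; The effect's horizontal scale derives from the skill's trace radius, so the visual follows the configured area, while height stays fixed.
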(event `self.SkillStart`
  (bind _returnvalue (/ (`.Radius_19_6BDBC5774B346A254DE606BFD88AD5E7` (break `/Game/RPGSystem/Blueprints/Structure/Skill/S_SkillTraceSettings` (`.TraceSettings_239_6436F7F74F429B5E93F83AB2033EF85B` (break `/Game/RPGSystem/Blueprints/Structure/Skill/S_Skill` (`self.SkillInfo`))))) 60.0))
  (`self.SpawnParticles` "/Game/RPGSystem/Particles/P_WirbelWind.P_WirbelWind" (`self.K2_GetActorRotation`) (`self.K2_GetActorLocation`) (0.0 0.0 0.0) (`KismetMathLibrary.MakeVector` _returnvalue _returnvalue 1.0) 999999.0 true self)
  (`parent.SkillStart`))

(fn `UserConstructionScript`
  (`parent.UserConstructionScript`))