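; Base AI character for RPG enemies, companions and minions, exposing its RPG system, drop, equipment and animation hooks to other systems.
; BPCRPGSystemAI events drive hit sounds and a floating HP/SP widget, created on damage or for slaves, optionally owner-only.
; Server Tick smoothly turns the living character toward its blackboard target or velocity.
; Death unpossesses it, ragdolls the mesh, stills it once settled and sets a random short lifespan.
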(event `OnSpChanged`
  (params (SP :type "Float (double-precision)") (MaxSP :type "Float (double-precision)") (FromSE :type Boolean))
  (bind _returnvalue (`KismetSystemLibrary.IsServer`))
  (bind ((`SP_70_7B08BD3D4DD5CE744876A4A2EB63058F` _sp) (`MaxSP_71_F40020B64C5A8ED80F1F718E65FE5701` _maxsp)) (break `/Game/RPGSystem/Blueprints/Structure/Player/S_Stats` (`.Stats_160_39D2053C4481A7FD69BEE0BA025AC4FB` (break `/Game/RPGSystem/Blueprints/Structure/Player/S_PlayerInfo` (`/Game/RPGSystem/Blueprints/BPC_RPGSystem.PlayerInfo` (`self.BPC_RPGSystem_AI`))))))
  ;[1 1 1] HealthBar Widget / HIt sound
  (`/Engine/EditorBlueprintResources/StandardMacros.IsValid` (`self.HealthBar`)
    (:`Is Valid`
      (message `/Game/RPGSystem/Blueprints/Interface/BPI_OverheadWidget.UpdateInfoSP` (`WidgetComponent.GetUserWidgetObject` (`self.HealthBar`)) (select `bool` _returnvalue :`false` SP :`true` _sp) (select `bool` _returnvalue :`false` MaxSP :`true` _maxsp)))))

(event `self.ReceiveBeginPlay`
  (bind _bpc_rpgsystem_ai (`self.BPC_RPGSystem_AI`))
  ;[1 1 1] BeginPlay - Major Update 3 - Changed
  (`|ExecutionSequence`
    (:`then_0`
      (add `/Game/RPGSystem/Blueprints/BPC_RPGSystem.OnDeath` (`self.BPC_RPGSystem_AI`) (`|CreateDelegate` :!event `OnDead`))
      (add `/Game/RPGSystem/Blueprints/BPC_RPGSystem.OnHPChanged` (`self.BPC_RPGSystem_AI`) (`|CreateDelegate` :!event `OnHpChanged`))
      (add `/Game/RPGSystem/Blueprints/BPC_RPGSystem.OnCompanionInit` _bpc_rpgsystem_ai (`|CreateDelegate` :!event `CreateHPSPWidget`))
      (add `/Game/RPGSystem/Blueprints/BPC_RPGSystem.OnMinionInit` _bpc_rpgsystem_ai (`|CreateDelegate` :!event `CreateHPSPWidget`))
      (add `/Game/RPGSystem/Blueprints/BPC_RPGSystem.OnSPChanged` _bpc_rpgsystem_ai (`|CreateDelegate` :!event `OnSpChanged`)))
    (:`then_1`
      (if (not (`KismetSystemLibrary.IsServer`))
        (`KismetSystemLibrary.Delay` 0.2)
        (`self.CreateHPSPWidget`)))
    (:`then_2`
      (`self.SetActorTickEnabled` true)
      (bind (_success _reference) (`self.GetRPGSystem`))
      (set `/Game/RPGSystem/Blueprints/BPC_RPGSystem.ForceDisableMovement` true _reference))))

(event `OnHpChanged`
  (params (HP :type "Float (double-precision)") (MaxHP :type "Float (double-precision)") (FromSE :type Boolean))
  (bind _returnvalue (`KismetSystemLibrary.IsServer`))
  (bind _mesh (`self.Mesh`))
  (bind ((`HP_68_883F47DD49C5298FBABCADAC0C04B9FA` _hp) (`MaxHP_69_86875F3049B9ECF13BADB3B89C5ED447` _maxhp)) (break `/Game/RPGSystem/Blueprints/Structure/Player/S_Stats` (`.Stats_160_39D2053C4481A7FD69BEE0BA025AC4FB` (break `/Game/RPGSystem/Blueprints/Structure/Player/S_PlayerInfo` (`/Game/RPGSystem/Blueprints/BPC_RPGSystem.PlayerInfo` (`self.BPC_RPGSystem_AI`))))))
  ;[1 1 1] HealthBar Widget / HIt sound
  (if (not FromSE)
    (`GameplayStatics.PlaySoundAtLocation` (`self.HitSound`) (`SceneComponent.K2_GetComponentLocation` (`self.Mesh`)) (struct) 1.0 1.0 0.0 null null null null))
  (if (not (`/Game/RPGSystem/Blueprints/BPC_RPGSystem.IsDead` (`self.BPC_RPGSystem_AI`)))
    (`/Engine/EditorBlueprintResources/StandardMacros.IsValid` (`self.HealthBar`)
      (:`Is Valid`
        _)
      (:`Is Not Valid`
        (`self.GetMeshRadius`)
        (`/Engine/EditorBlueprintResources/StandardMacros.IsValid` _mesh
          (:`Is Valid`
            (bind _returnvalue_2 (`AddComponent|NODE_AddWidgetComponent-0` :`RelativeTransform` (`KismetMathLibrary.MakeTransform` (`KismetMathLibrary.MakeVector` 0.0 0.0 (* (.z (`.BoxExtent` (`KismetSystemLibrary.GetComponentBounds` _mesh))) 1.0)))))
            (set `self.HealthBar` _returnvalue_2)))))
    (message `/Game/RPGSystem/Blueprints/Interface/BPI_OverheadWidget.UpdateInfoHP` (`WidgetComponent.GetUserWidgetObject` (`self.HealthBar`)) (select `bool` _returnvalue :`false` HP :`true` _hp) (select `bool` _returnvalue :`false` MaxHP :`true` _maxhp))))

(event `CreateHPSPWidget`
  (bind _bpc_rpgsystem_ai (`self.BPC_RPGSystem_AI`))
  (bind _slavefloatinghud_owneronly (`self.SlaveFloatingHUD_OwnerOnly`))
  (bind (_hp _maxhp) (`/Game/RPGSystem/Blueprints/BPC_RPGSystem.GetHP` (`self.BPC_RPGSystem_AI`)))
  (bind _returnvalue (== (`ActorComponent.GetOwner` (`/Game/RPGSystem/Blueprints/BPC_RPGSystem.SlaveMaster` (`self.BPC_RPGSystem_AI`))) (`GameplayStatics.GetPlayerCharacter` 0)))
  ;[1 1 1] BeginPlay - Major Update 3 - Changed
  (`/Engine/EditorBlueprintResources/StandardMacros.IsValid` (`self.HealthBar`)
    (:`Is Not Valid`
      (if (`/Game/RPGSystem/Blueprints/BPC_RPGSystem.IsCompanion` _bpc_rpgsystem_ai)
        (if _slavefloatinghud_owneronly
          (`/Engine/EditorBlueprintResources/StandardMacros.IsValid` (`GameplayStatics.GetPlayerCharacter` 0)
            (:`Is Valid`
              (if _returnvalue
                (bind _returnvalue_2 (`AddComponent|NODE_AddWidgetComponent-1` :`RelativeTransform` (`KismetMathLibrary.MakeTransform` (`KismetMathLibrary.MakeVector` 0.0 0.0 (* (.z (`.BoxExtent` (`KismetSystemLibrary.GetComponentBounds` (`self.Mesh`)))) 1.75))) :!label _label))
                (set `self.HealthBar` _returnvalue_2))))
          (else
            (goto _label)))
        (elif (`/Game/RPGSystem/Blueprints/BPC_RPGSystem.IsMinion` _bpc_rpgsystem_ai)
          (if _slavefloatinghud_owneronly
            (`/Engine/EditorBlueprintResources/StandardMacros.IsValid` (`GameplayStatics.GetPlayerCharacter` 0)
              (:`Is Valid`
                (if _returnvalue
                  (bind _returnvalue_3 (`AddComponent|NODE_AddWidgetComponent-2` :`RelativeTransform` (`KismetMathLibrary.MakeTransform` (`KismetMathLibrary.MakeVector` 0.0 0.0 (* (.z (`.BoxExtent` (`KismetSystemLibrary.GetComponentBounds` (`self.Mesh`)))) 1.0))) :!label _label_2))
                  (set `self.HealthBar` _returnvalue_3))))
            (else
              (goto _label_2)))
          (elif (< _hp _maxhp)
            (`self.OnHpChanged` _hp _maxhp)))))))

(event `self.ReceiveDestroyed`
  (bind _healthbar (`self.HealthBar`))
  ;[1 1 1] Destroyed
  (`/Engine/EditorBlueprintResources/StandardMacros.IsValid` _healthbar
    (:`Is Valid`
      (`ActorComponent.K2_DestroyComponent` _healthbar))))

(event `/Game/RPGSystem/Blueprints/Interface/BPI_Interaction.SelectInteractable`
  (params (Selected :type Boolean))
  ;[1 1 1] Select Interactable
  (`PrimitiveComponent.SetRenderCustomDepth` (`self.Mesh`) Selected))

(event `self.VisualEquipmentDestroyComponent`
  (params (Component :type "ActorComponent Object Reference"))
  ;[1 1 1] Visual Equipment
  (`ActorComponent.K2_DestroyComponent` Component))

(event `self.ReceiveUnpossessed`
  (params (OldController :type "Controller Object Reference"))
  (`self.SetLifeSpan` OldController 0.01))

(event `self.VisualEquipmentDestroyComponents`
  (params (Components :type "Array of ActorComponent Object Reference (by ref)"))
  ;[1 1 1] Visual Equipment
  (`ActorComponent.K2_DestroyComponent` Components))

(event `ActivateRagdoll`
  (params (Impulse_Struct :type "/Game/RPGSystem/Blueprints/Structure/Skill/S_Impulse Structure"))
  (bind _capsulecomponent (`self.CapsuleComponent`))
  ;[1 1 1] Ragdoll
  (`PrimitiveComponent.SetCollisionEnabled` (`self.Mesh`) "PhysicsOnly")
  (`/Game/RPGSystem/Blueprints/BPC_RPGSystem.EnableRagdoll` (`self.BPC_RPGSystem_AI`) (`self.Mesh`) Impulse_Struct)
  (`ActorComponent.Deactivate` (`self.CharacterMovement`))
  (`ActorComponent.Deactivate` (`self.BPC_RPGSystem_AI`))
  (`ActorComponent.Deactivate` (`self.CapsuleComponent`))
  (`self.SetActorTickEnabled` false)
  (`ActorComponent.SetComponentTickEnabled` (`self.BPC_RPGSystem_AI`) false)
  (`ActorComponent.SetComponentTickEnabled` (`self.CharacterMovement`) false)
  (`KismetSystemLibrary.RetriggerableDelay` 0.5)
  (`/Engine/EditorBlueprintResources/StandardMacros.IsValid` _capsulecomponent
    (:`Is Valid`
      (`ActorComponent.K2_DestroyComponent` _capsulecomponent))
    (:`Is Not Valid`
      _))
  (`/Engine/EditorBlueprintResources/StandardMacros.IsValid` (`self.Mesh`) :!label _label_3
    (:`Is Valid`
      (if (<= (`KismetMathLibrary.VSize` (`SceneComponent.GetComponentVelocity` (`self.Mesh`))) 1.0)
        (`/Engine/EditorBlueprintResources/StandardMacros.DoOnce` false
          (:`Completed`
            (`PrimitiveComponent.SetPhysicsLinearVelocity` (`self.Mesh`) (0.0 0.0 0.0) false "None")))
        (else
          (`KismetSystemLibrary.Delay` 0.5)
          (goto _label_3))))))

(event `OnDeathTimer`
  ;[1 1 1] OnDeath
  (`self.SetLifeSpan` (`KismetMathLibrary.RandomFloatInRange` 8.0 10.0)))

(event `OnDead`
  (params (Attacker :type "/Game/RPGSystem/Blueprints/BPC_RPGSystem Object Reference") (Impulse :type "/Game/RPGSystem/Blueprints/Structure/Skill/S_Impulse Structure") (Victim :type "/Game/RPGSystem/Blueprints/BPC_RPGSystem Object Reference"))
  (bind _bpc_rpgsystem_ai (`self.BPC_RPGSystem_AI`))
  ;[1 1 1] OnDeath
  (`/Engine/EditorBlueprintResources/StandardMacros.IsValid` (`self.HealthBar`)
    (:`Is Valid`
      (`ActorComponent.K2_DestroyComponent` (`self.HealthBar`)))
    (:`Is Not Valid`
      _))
  (`self.SetActorTickEnabled` false)
  (set `/Game/RPGSystem/Blueprints/BPC_RPGSystem.IsDead` true _bpc_rpgsystem_ai)
  (`/Game/RPGSystem/Blueprints/BPC_RPGSystem.InterruptCast` _bpc_rpgsystem_ai)
  (`ActorComponent.SetComponentTickEnabled` _bpc_rpgsystem_ai false)
  (`/Engine/EditorBlueprintResources/ActorMacros.Switch Has Authority`
    (:`Authority`
      (`Controller.UnPossess` (`self.GetController`)))
    (:`Remote`
      _))
  (`NavMovementComponent.StopActiveMovement` (`self.CharacterMovement`))
  (`self.ActivateRagdoll` Impulse)
  (`GameplayStatics.PlaySoundAtLocation` (`self.DyingSound`) (`SceneComponent.K2_GetComponentLocation` (`self.Mesh`)) (struct) 1.0 1.0 0.0 null null null null)
  (`self.OnDeathTimer`))

(event `/Game/RPGSystem/Blueprints/Interface/BPI_RPGAnimation.SetAnimationState`
  (params (State :type "/Game/RPGSystem/Blueprints/Enum/Item/E_ItemType Enum" :default "NewEnumerator10"))
  ;[1 1 1] Animations
  (set `self.AnimationState` State))

(event `/Game/RPGSystem/Blueprints/Interface/BPI_RPGAnimation.PlayHitAnimation`
  (params (Impulse :type "/Game/RPGSystem/Blueprints/Structure/Skill/S_Impulse Structure"))
  ;[1 1 1] Animations
  (message `/Game/RPGSystem/Blueprints/Interface/BPI_RPGAnimation.PlayHitAnimation` (`SkeletalMeshComponent.GetAnimInstance` (`self.Mesh`)) Impulse))

(event `/Game/RPGSystem/Blueprints/Interface/BPI_RPGAnimation.PlaySkillAnimation`
  (params (`State ` :type "/Game/RPGSystem/Blueprints/Enum/Skill/E_AnimationState Enum" :default "NewEnumerator0") (`SkillID ` :type Name) (`Speed ` :type "Float (double-precision)") (`Time ` :type "Float (double-precision)"))
  (bind _mesh (`self.Mesh`))
  ;[1 1 1] Animations
  (if (`KismetSystemLibrary.IsValid` _mesh)
    (message `/Game/RPGSystem/Blueprints/Interface/BPI_RPGAnimation.PlaySkillAnimation` (`SkeletalMeshComponent.GetAnimInstance` _mesh) `State ` `SkillID ` `Speed ` `Time `)))

(event `self.ReceiveTick`
  (params (DeltaSeconds :type "Float (single-precision)"))
  (bind _returnvalue (`self.GetVelocity`))
  (bind _bpc_rpgsystem_ai (`self.BPC_RPGSystem_AI`))
  (bind _returnvalue_2 (`AIBlueprintHelperLibrary.GetBlackboard` (`AIBlueprintHelperLibrary.GetAIController` self)))
  (bind _returnvalue_3 (> (`KismetMathLibrary.VSize` _returnvalue) 10.0))
  (bind _returnvalue_4 (+ (`self.K2_GetActorLocation`) (* _returnvalue 10.0)))
  (bind _returnvalue_5 (`BlackboardComponent.GetValueAsObject` _returnvalue_2 "Target"))
  ;[1 1 1] Smooth Rotation
  (if (and (`KismetSystemLibrary.IsServer`) (not (`/Game/RPGSystem/Blueprints/BPC_RPGSystem.IsDead` (`self.BPC_RPGSystem_AI`))))
    (set `self.Falling` (`NavMovementComponent.IsFalling` (`self.CharacterMovement`)))
    (if (`/Game/RPGSystem/Blueprints/BPC_RPGSystem.DisableMovement` _bpc_rpgsystem_ai)
      (`|ExecutionSequence`
        (:`then_0`
          (`/Engine/EditorBlueprintResources/StandardMacros.Gate` false :!label _label_4
            (:`Exit`
              (`MovementComponent.StopMovementImmediately` (`self.CharacterMovement`))
              (goto _label_4 :!via `Close`))))
        (:`then_1`
          _))
      (else
        (`|ExecutionSequence`
          (:`then_0`
            _)
          (:`then_1`
            (goto _label_4 :!via `Open`)))))
    (if (not (`/Game/RPGSystem/Blueprints/BPC_RPGSystem.DisableAttacking` _bpc_rpgsystem_ai))
      (`/Engine/EditorBlueprintResources/StandardMacros.IsValid` (`AIBlueprintHelperLibrary.GetAIController` self)
        (:`Is Valid`
          (if (`BlackboardComponent.GetValueAsBool` _returnvalue_2 "HasTarget")
            (if (`self.LockLookAtTargetClose`)
              (bind _radius (message `/Game/RPGSystem/Blueprints/Interface/BPI_RPGSystem.GetMeshRadius` _returnvalue_5))
              (if (< (`/Game/RPGSystem/Blueprints/Interface/BPL_RPGSystem.GetDistanceXY` (`self.K2_GetActorLocation`) (`BlackboardComponent.GetValueAsVector` _returnvalue_2 "TargetLocation")) (+ _radius (* (`CapsuleComponent.GetScaledCapsuleRadius` (`self.CapsuleComponent`)) 3.0) (+ (`/Game/RPGSystem/Blueprints/BPC_RPGSystem.GetSkillAttackRangeUnits` (`self.BPC_RPGSystem_AI`)) 350.0)))
                (bind (_success _reference) (message `/Game/RPGSystem/Blueprints/Interface/BPI_RPGSystem.GetRPGSystem` _returnvalue_5 :!label _label_5))
                (if _success
                  (set `self.LookAt` (`self.K2_GetActorLocation` (`ActorComponent.GetOwner` _reference)))
                  (`/Game/RPGSystem/Blueprints/BPC_RPGSystem_AI.SetSmoothRotationToTarget` (`self.BPC_RPGSystem_AI`) (`self.LookAt`) 4.0 DeltaSeconds :!label _label_6))
                (else
                  (if _returnvalue_3 :!label _label_7
                    (set `self.LookAt` _returnvalue_4)
                    (goto _label_6)
                    (else
                      (goto _label_5)))))
              (else
                (goto _label_7)))
            (elif _returnvalue_3
              (set `self.LookAt` _returnvalue_4)
              (goto _label_6))))))))

(event `/Game/RPGSystem/Blueprints/Interface/BPI_RPGAnimation.StopSkillAnimation`
  ;[1 1 1] Animations
  (`self.StopAnimMontage` (`self.GetCurrentMontage`)))

(fn `GetAnimationState`
  (returns (State :type "/Game/RPGSystem/Blueprints/Enum/Item/E_ItemType Enum"))
  (return (`self.AnimationState`)))

(fn `GetCapsuleHalfHeight`
  (returns (HalfHeight :type "Float (double-precision)"))
  (return (`CapsuleComponent.GetScaledCapsuleHalfHeight` (`self.CapsuleComponent`))))

(fn `GetDropSystemComponent`
  (returns (Success :type Boolean) (Component :type "/Game/RPGSystem/Blueprints/BPC_DropSystem Object Reference"))
  (return true (`self.BPC_DropSystem`)))

(fn `GetEnemyInfo`
  (returns (Succes :type Boolean) (MonsterID :type Name) (Info :type "/Game/RPGSystem/Blueprints/Structure/Monster/S_Monster Structure") (CustomVariables :type "/Game/RPGSystem/Blueprints/Structure/S_ArrayOf_FName Structure") (CustomVariablesPrivate :type "/Game/RPGSystem/Blueprints/Structure/S_ArrayOf_FName Structure"))
  (locals (VarCustomVariables :type "Array of Name") (VarCustomVariablesPrivate :type "Array of Name"))
  (bind _bpc_rpgsystem_ai (`self.BPC_RPGSystem_AI`))
  (bind _bpc_rpgsystem_ai_2 (`self.BPC_RPGSystem_AI`))
  (set `local.VarCustomVariables` (`/Game/RPGSystem/Blueprints/BPC_RPGSystem_AI.CustomVariables` _bpc_rpgsystem_ai))
  (set `local.VarCustomVariablesPrivate` (`/Game/RPGSystem/Blueprints/BPC_RPGSystem_AI.CustomVariablesPrivate` _bpc_rpgsystem_ai))
  (for _array_element (`/Game/RPGSystem/Blueprints/BPC_RPGSystem_AI.CustomVariablesTags` (`self.BPC_RPGSystem_AI`))
    (`KismetArrayLibrary.Array_Add` (`local.VarCustomVariables`) (`BlueprintGameplayTagLibrary.GetTagName` _array_element)))
  (for _array_element_2 (`/Game/RPGSystem/Blueprints/BPC_RPGSystem_AI.CustomVariablesTagsPrivate` (`self.BPC_RPGSystem_AI`))
    (`KismetArrayLibrary.Array_Add` (`local.VarCustomVariablesPrivate`) (`BlueprintGameplayTagLibrary.GetTagName` _array_element_2)))
  (return true (`/Game/RPGSystem/Blueprints/BPC_RPGSystem_AI.MonsterID` _bpc_rpgsystem_ai_2) (`/Game/RPGSystem/Blueprints/BPC_RPGSystem_AI.EnemyInfo` _bpc_rpgsystem_ai_2) (make `/Game/RPGSystem/Blueprints/Structure/S_ArrayOf_FName` (`local.VarCustomVariables`)) (make `/Game/RPGSystem/Blueprints/Structure/S_ArrayOf_FName` (`local.VarCustomVariablesPrivate`))))

(fn `GetInteractInfo`
  (params (RPGSystem :type "/Game/RPGSystem/Blueprints/BPC_RPGSystem Object Reference"))
  (returns (Success :type Boolean) (Action :type "/Game/RPGSystem/Blueprints/Enum/Interact/E_InteractAction Enum"))
  (return true "NewEnumerator2"))

(fn `GetMeshRadius`
  (returns (Radius :type "Float (double-precision)"))
  (bind _capsulecomponent (`self.CapsuleComponent`))
  (if (`KismetSystemLibrary.IsValid` _capsulecomponent)
    (return (* (`CapsuleComponent.GetScaledCapsuleRadius` _capsulecomponent) 1.0))
    (else
      (return 0.0))))

(fn `GetMovementSpeed`
  (returns (Speed :type "Float (double-precision)"))
  (return (`CharacterMovementComponent.MaxWalkSpeed` (`self.CharacterMovement`))))

(fn `GetMoveToEndDestination`
  (returns (Success :type Boolean) (WorldLocation :type "Vector Structure"))
  (return false (0.0 0.0 0.0)))

(fn `GetPlayerSkeletalMesh`
  (returns (Success :type Boolean) (Component :type "SkeletalMeshComponent Object Reference"))
  (bind _mesh (`self.Mesh`))
  (return (`KismetSystemLibrary.IsValid` _mesh) _mesh))

(fn `GetRPGSystem`
  (returns (Success :type Boolean) (Reference :type "/Game/RPGSystem/Blueprints/BPC_RPGSystem Object Reference"))
  (bind _bpc_rpgsystem_ai (`self.BPC_RPGSystem_AI`))
  (return (not (`/Game/RPGSystem/Blueprints/BPC_RPGSystem.IsDead` _bpc_rpgsystem_ai)) _bpc_rpgsystem_ai))

(fn `GetRPGSystemAI`
  (returns (Success :type Boolean) (Reference :type "/Game/RPGSystem/Blueprints/BPC_RPGSystem_AI Object Reference"))
  (return true (`self.BPC_RPGSystem_AI`)))

(fn `GetScreenTooltipInfo`
  (params (RPGSystem :type "/Game/RPGSystem/Blueprints/BPC_RPGSystem Object Reference")))

(fn `GetWorldTooltipInfo`
  (returns (Success :type Boolean) (Interactable :type Boolean) (Text :type Text) (Color :type "LinearColor Structure") (Offset :type "Vector Structure"))
  (return false false "" (struct) (0.0 0.0 0.0)))

(fn `IsDualWield`
  (returns (Success :type Boolean))
  (bind _bpc_rpgsystem_ai (`self.BPC_RPGSystem_AI`))
  (`/Engine/EditorBlueprintResources/StandardMacros.IsValid` _bpc_rpgsystem_ai
    (:`Is Valid`
      (return (`/Game/RPGSystem/Blueprints/BPC_RPGSystem.IsDualWield` _bpc_rpgsystem_ai)))
    (:`Is Not Valid`
      (return false))))

(fn `IsFalling`
  (returns (Falling :type Boolean))
  (return (`self.Falling`)))

(fn `IsTwohanded`
  (returns (Success :type Boolean))
  (bind _bpc_rpgsystem_ai (`self.BPC_RPGSystem_AI`))
  (`/Engine/EditorBlueprintResources/StandardMacros.IsValid` _bpc_rpgsystem_ai
    (:`Is Valid`
      (return (`/Game/RPGSystem/Blueprints/BPC_RPGSystem.IsTwoHanded` _bpc_rpgsystem_ai)))
    (:`Is Not Valid`
      (return false))))

(fn `SetMeshRotation`
  (params (Target :type "Vector Structure (by ref)") (Rate :type "Float (double-precision)") (DeltaTime :type "Float (double-precision)"))
  (bind _mesh (`self.Mesh`))
  (bind _returnvalue (`SceneComponent.K2_GetComponentRotation` _mesh))
  (`SceneComponent.K2_SetWorldRotation` (`self.Mesh`) (`KismetMathLibrary.RInterpTo_Constant` _returnvalue (`KismetMathLibrary.ComposeRotators` (`KismetMathLibrary.MakeRotator` (.roll (`KismetMathLibrary.FindLookAtRotation` (`SceneComponent.K2_GetComponentLocation` _mesh) Target)) (.pitch _returnvalue) (.yaw (`KismetMathLibrary.FindLookAtRotation` (`SceneComponent.K2_GetComponentLocation` _mesh) Target))) (struct :`Yaw` -90.0)) DeltaTime (* Rate 100.0)) false true))

(fn `SetMovementSpeed`
  (params (ToDefault :type Boolean) (Speed :type "Float (double-precision)"))
  (set `CharacterMovementComponent.MaxWalkSpeed` (`KismetMathLibrary.SelectFloat` 600.0 Speed ToDefault) (`self.CharacterMovement`)))

(fn `UserConstructionScript`)

(fn `VisualEquipmentAddSkeletalMeshComponent`
  (returns (Component :type "SkeletalMeshComponent Object Reference"))
  (bind _returnvalue (`AddComponent|NODE_AddSkeletalMeshComponent-1`))
  (return _returnvalue))

(fn `VisualEquipmentAddStaticMeshComponent`
  (returns (Component :type "StaticMeshComponent Object Reference"))
  (bind _returnvalue (`AddComponent|NODE_AddStaticMeshComponent-1`))
  (return _returnvalue))