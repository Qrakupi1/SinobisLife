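; BP_Comp_Manfred is a companion character Blueprint in the RPG system that supplies mesh hooks for visual equipment.
; It creates skeletal and static mesh components on request for equipment visuals and reports its own Mesh as the skeletal mesh.
; The construction script only calls the parent, leaving a random BodyColor dynamic material branch disconnected.
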(fn `GetPlayerSkeletalMesh`
  (returns (Success :type Boolean) (Component :type "SkeletalMeshComponent Object Reference"))
  (return true (`self.Mesh`)))

(fn `UserConstructionScript`
  (`parent.UserConstructionScript`))

(fn `VisualEquipmentAddSkeletalMeshComponent`
  (returns (Component :type "SkeletalMeshComponent Object Reference"))
  (bind _returnvalue (`AddComponent|NODE_AddSkeletalMeshComponent-0`))
  (return _returnvalue))

(fn `VisualEquipmentAddStaticMeshComponent`
  (returns (Component :type "StaticMeshComponent Object Reference"))
  (bind _returnvalue (`AddComponent|NODE_AddStaticMeshComponent-0`))
  (return _returnvalue))