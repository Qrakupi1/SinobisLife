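; BP_SharinganDodge_Body is an afterimage actor for a Sharingan dodge skill, showing a fading frozen copy of a character's pose.
; SpawnAfterimage applies one dynamic instance of M_SharinganDodge_Body to the poseable mesh's material slots, counted from ModelRef, then copies that skeletal component's current pose.
; A timeline drives the material's Opacity parameter, and the actor destroys itself when the timeline finishes.
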(event `SpawnAfterimage`
  (bind _returnvalue (`KismetMaterialLibrary.CreateDynamicMaterialInstance` "/Game/RPGSystem/Models/Mannequin/Materials/M_SharinganDodge_Body.M_SharinganDodge_Body"))
  (set `self.AfterimageMaterial` _returnvalue)
  (for _index (range (`PrimitiveComponent.GetNumMaterials` (`self.ModelRef`)))
    (`PrimitiveComponent.SetMaterial` (`self.PoseableMesh`) _index (`self.AfterimageMaterial`)))
  (`PoseableMeshComponent.CopyPoseFromSkeletalComponent` (`self.PoseableMesh`) (`self.ModelRef`))
  (bind (_direction _opacity) (`Timeline|AfterimageTimeline`)
    (:`Update`
      (`MaterialInstanceDynamic.SetScalarParameterValue` (`self.AfterimageMaterial`) "Opacity" _opacity))
    (:`Finished`
      (`self.K2_DestroyActor`))))

(fn `UserConstructionScript`)