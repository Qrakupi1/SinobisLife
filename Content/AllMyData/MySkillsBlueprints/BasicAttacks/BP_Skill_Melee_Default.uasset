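; Default melee basic-attack skill Blueprint that checks for enemies around its owner when the skill starts.
; SkillStart runs a zero-length multi sphere trace on the Visibility channel at the owner's location, with debug drawing.
; Each hit that casts to BP_Enemy_Base calls OnForceExecuteSkill on the skill owner, passing the skill itself rather than the enemy.
; SkillEnd, ForceExecuteSkill and server animation calls are left unconnected.
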(event `self.SkillStart`
  (bind _returnvalue (`self.K2_GetActorLocation` (`self.GetOwner`)))
  (bind (_outhits _returnvalue_2) (`KismetSystemLibrary.SphereTraceMulti` :`Start` _returnvalue :`End` _returnvalue :`Radius` 1000.0 :`TraceChannel` "TraceTypeQuery1" :`DrawDebugType` "ForDuration"))
  (if _returnvalue_2
    (for _array_element _outhits
      (cast `/Game/RPGSystem/Blueprints/AI/BP_Enemy_Base` (`.HitActor` (`GameplayStatics.BreakHitResult` _array_element)))
      (`/Game/RPGSystem/Blueprints/BPC_RPGSystem.OnForceExecuteSkill` (`self.SkillOwner`) self))))

(fn `UserConstructionScript`
  (`parent.UserConstructionScript`))